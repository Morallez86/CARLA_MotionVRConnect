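; VR-drivable Mercedes CCC vehicle Blueprint that maps player input to vehicle movement and drives a YawController with motion values.
; BeginPlay adjusts the camera for an HMD, links a cylinder text widget and plays a startup sound before enabling throttle and RPM-driven engine audio.
; Axis inputs set throttle, brake and steering, then feed smoothed, speed-scaled roll and pitch to the YawController.
; A toggle action switches between reverse and first gear.
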(event EventBeginPlay
  (bind _sounds (Variables|Default|GetSounds))
  (Utilities|FlowControl|Sequence
    (:then_0
      (Utilities|FlowControl|Delay 0.05)
      (if (Class|HeadMountedDisplayFunctionLibrary|IsHeadMountedDisplayEnabled)
        (Class|HeadMountedDisplayFunctionLibrary|SetTrackingOrigin "Eye")
        (Transformation|SetRelativeLocation (Variables|Default|GetCameraRoot) "11.000000,-30.000000,113.000000" false false)))
    (:then_1
      (bind _ascylinder_text (Utilities|Casting|CastToCylinder_Text (UserInterface|GetUserWidgetObject (Variables|Default|GetWidget))))
      (Variables|/Game/Carla/Blueprints/Vehicles/MercedesCCC_VR/HUD/Cylinder_Text.Cylinder_Text_C|SetOwning%20Actor _ascylinder_text self))
    (:then_2
      (Audio|Components|Audio|SetSound _sounds "/Game/Carla/Blueprints/Vehicles/MercedesCCC_VR/Sound/engine-start-86242.engine-start-86242")
      (Audio|Components|Audio|Play _sounds 0.0)
      (Utilities|FlowControl|Delay 3.2)
      (Variables|Default|SetEngineOn true))))

(event EventTick
  (params (DeltaSeconds :type Float%20%28single-precision%29))
  (bind _vehiclemovement (Variables|Default|GetVehicleMovement))
  (bind _engine (Variables|Default|GetEngine))
  (bind _returnvalue (Class|WheeledVehicleMovementComponent|GetEngineRotationSpeed _vehiclemovement))
  (if (Variables|Default|GetEngineOn)
    (if (< _returnvalue 6e+02)
      (Audio|Parameter|SetFloatParameter _engine "RPM" 6e+02 :!class /Script/Engine.AudioComponent)
      (else
        (Audio|Parameter|SetFloatParameter _engine "RPM" _returnvalue :!class /Script/Engine.AudioComponent)))))

(event Input|ActionEvents|InputActionToggleReverse
  (params (Key :type Key%20Structure))
  (bind _vehiclemovement (Variables|Default|GetVehicleMovement))
  (:Pressed
    (bind _output_get (Variables|Default|SetIsReverse (not (Variables|Default|GetIsReverse))))
    (if _output_get
      (Class|WheeledVehicleMovementComponent|SetTargetGear _vehiclemovement -1 false)
      (else
        (Class|WheeledVehicleMovementComponent|SetTargetGear _vehiclemovement 1 false)))))

(event Input|AxisEvents|InputAxisMoveRight
  (params (AxisValue :type Float%20%28single-precision%29))
  (Class|WheeledVehicleMovementComponent|SetSteeringInput (Variables|Default|GetVehicleMovement) AxisValue)
  (bind _newparam3 (CallFunction|GetRotationfromAxis AxisValue (stale Input|AxisEvents|InputAxisMoveFoward AxisValue) (stale Input|AxisEvents|InputAxisBrake AxisValue)))
  (Class|YawController|UpdateMotionValues (Variables|Default|GetYawController) _newparam3))

(event Input|AxisEvents|InputAxisMoveFoward
  (params (AxisValue :type Float%20%28single-precision%29))
  (if (Variables|Default|GetEngineOn)
    (Class|WheeledVehicleMovementComponent|SetThrottleInput (Variables|Default|GetVehicleMovement) AxisValue)
    (bind _newparam3 (CallFunction|GetRotationfromAxis (stale Input|AxisEvents|InputAxisMoveRight AxisValue) AxisValue (stale Input|AxisEvents|InputAxisBrake AxisValue)))
    (Class|YawController|UpdateMotionValues (Variables|Default|GetYawController) _newparam3)))

(event Input|AxisEvents|InputAxisBrake
  (params (AxisValue :type Float%20%28single-precision%29))
  (Class|WheeledVehicleMovementComponent|SetBrakeInput (Variables|Default|GetVehicleMovement) AxisValue)
  (bind _newparam3 (CallFunction|GetRotationfromAxis (stale Input|AxisEvents|InputAxisMoveRight AxisValue) (stale Input|AxisEvents|InputAxisMoveFoward AxisValue) AxisValue))
  (Class|YawController|UpdateMotionValues (Variables|Default|GetYawController) _newparam3))

(fn ConstructionScript
  (|CallParentFunction))

(fn GetRotationfromAxis
  (params (Turn :type Float%20%28single-precision%29) (Thrust :type Float%20%28single-precision%29) (Brake :type Float%20%28single-precision%29))
  (bind _vehiclemovement (Variables|Default|GetVehicleMovement))
  (bind _returnvalue (Class|WheeledVehicleMovementComponent|GetForwardSpeed _vehiclemovement))
  (bind _returnvalue_2 (* _returnvalue 0.036))
  (bind _returnvalue_3 (Math|Float|Truncate _returnvalue_2))
  (bind _returnvalue_4 (Math|Integer|Clamp(Integer) _returnvalue_3 0 10))
  (bind _output_get (Variables|Default|SetCurrentXRotation (Math|Interpolation|FInterpTo (Variables|Default|GetCurrentXRotation) (* _returnvalue_4 Turn) (Utilities|Time|GetWorldDeltaSeconds) 1.0)))
  (bind _output_get_2 (Variables|Default|SetCurrentYRotation (Math|Interpolation|FInterpTo (Variables|Default|GetCurrentYRotation) (* _returnvalue_4 (- Thrust Brake)) (Utilities|Time|GetWorldDeltaSeconds) 1.0)))
  (return (Math|Rotator|MakeRotator _output_get _output_get_2 0.0)))